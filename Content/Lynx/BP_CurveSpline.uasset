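; BP_CurveSpline is a spline path for the Lynx character, with begin and end triggers that start and stop spline movement.
; While tracking, Tick measures the moving player capsule's distance to the nearest spline point and flags when it crosses min or max bounds, printing debug text.
; PositionToSpline can pull the capsule halfway toward the spline when out of bounds, but nothing in this file calls it.
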(event `BeginSpline`
  (bind _player_ref (`self.Player Ref`))
  (set `/Game/Lynx/BP_LynxCharacter.InSpline` true _player_ref)
  (set `/Game/Lynx/BP_LynxCharacter.CurveSplineRef` self _player_ref)
  (set `self.StartTick` true))

(event `self.ReceiveBeginPlay`
  (bind _asbp_lynx_character (cast `/Game/Lynx/BP_LynxCharacter` (`GameplayStatics.GetPlayerCharacter` 0)))
  (set `self.Player Ref` _asbp_lynx_character))

(event `EndSpline`
  (bind _player_ref (`self.Player Ref`))
  (set `/Game/Lynx/BP_LynxCharacter.InSpline` false _player_ref)
  (set `/Game/Lynx/BP_LynxCharacter.CurveSplineRef` null _player_ref)
  (set `self.StartTick` false)
  (set `self.End` true)
  (`KismetSystemLibrary.PrintString` "Overlap end" true true (struct :`R` 1.0 :`G` 0.058055 :`A` 1.0)))

(event `self.ReceiveTick`
  (params (DeltaSeconds :type "Float (single-precision)"))
  (bind _player_ref (`self.Player Ref`))
  (bind _movingaround (`/Game/Lynx/BP_LynxCharacter.MovingAround` _player_ref))
  ;[1 1 1] Adjust bounds here
  (if (`self.StartTick`)
    (if (`/Game/Lynx/BP_LynxCharacter.InSpline` _player_ref)
      (if _movingaround
        (bind _distance (`self.CalcDis`))
        (`self.CalcBounds` _distance))
      (elif _movingaround
        (bind _distance_2 (`self.CalcDis`))
        (`self.CalcBounds` _distance_2)))))

(event `self.SplineBegin.OnComponentBeginOverlap`
  (params (OverlappedComponent :type "PrimitiveComponent Object Reference") (OtherActor :type "Actor Object Reference") (OtherComp :type "PrimitiveComponent Object Reference") (OtherBodyIndex :type Integer) (bFromSweep :type Boolean) (SweepResult :type "HitResult Structure (by ref)"))
  (bind _player_ref (`self.Player Ref`))
  (if (== OtherActor _player_ref)
    (`/Game/Lynx/BP_LynxCharacter.MoveAlongSpline` _player_ref)
    (set `self.StartTick` true)))

(event `self.SplineEnd.OnComponentBeginOverlap`
  (params (OverlappedComponent :type "PrimitiveComponent Object Reference") (OtherActor :type "Actor Object Reference") (OtherComp :type "PrimitiveComponent Object Reference") (OtherBodyIndex :type Integer) (bFromSweep :type Boolean) (SweepResult :type "HitResult Structure (by ref)"))
  (if (== OtherActor (`self.Player Ref`))
    (`self.EndSpline`)))

(fn `CalcBounds`
  (params (Distance :type "Float (double-precision)"))
  (if (>= Distance (`self.MaxBound`))
    (set `self.BoundCrossed` true)
    (`KismetSystemLibrary.PrintString` "BoundCrossedYMax" true true (struct :`R` 1.0 :`G` 0.046773 :`A` 1.0))
    (elif (<= Distance (`self.MinBound`))
      (set `self.BoundCrossed` true)
      (`KismetSystemLibrary.PrintString` "BoundCrossedYMin" true true (struct :`R` 1.0 :`G` 0.046773 :`A` 1.0))
      (else
        (set `self.BoundCrossed` false)
        (`KismetSystemLibrary.PrintString` "In Bounds" true true (struct :`R` 0.053398 :`G` 1.0 :`A` 1.0))))))

(fn `CalcDis`
  (returns (Distance :type "Float (double-precision)"))
  (bind _returnvalue (`SceneComponent.K2_GetComponentLocation` (`Character.CapsuleComponent` (`self.Player Ref`))))
  (bind _returnvalue_2 (`KismetMathLibrary.Vector_Distance` (`SplineComponent.FindLocationClosestToWorldLocation` (`self.Spline`) _returnvalue "World") _returnvalue))
  (`KismetSystemLibrary.PrintString` (`KismetStringLibrary.Conv_DoubleToString` _returnvalue_2))
  (return _returnvalue_2))

(fn `PositionToSpline`
  (bind _capsulecomponent (`Character.CapsuleComponent` (`self.Player Ref`)))
  (bind _returnvalue (`SceneComponent.K2_GetComponentLocation` (`Character.CapsuleComponent` (`self.Player Ref`))))
  (if (`self.BoundCrossed`)
    (`SceneComponent.K2_SetWorldLocation` _capsulecomponent (`KismetMathLibrary.VLerp` (`SplineComponent.FindLocationClosestToWorldLocation` (`self.Spline`) _returnvalue "World") _returnvalue 0.5) false false)
    (else
      (`SceneComponent.K2_SetWorldLocation` _capsulecomponent _returnvalue false false))))

(fn `UserConstructionScript`)